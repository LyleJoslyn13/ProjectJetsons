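; BP_Bounce is a short-lived, one-use bounce actor that launches the main character upward.
; On Box overlap it compares the other actor's class to Character, then casts to MainCharacter, adds upward launch velocity and destroys itself; a class mismatch prints a debug string.
; From BeginPlay, a next-tick delay loop accumulates delta time and destroys the actor once MaxLifeTime is reached, standing in for Event Tick.
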(event `self.ReceiveBeginPlay`
  (bind _output_get (set `self.currentLifeTime` (+ (* (`GameplayStatics.GetWorldDeltaSeconds`) 1.0) (`self.currentLifeTime`)) :!label _label))
  (if (>= _output_get (`self.maxLifeTime`))
    (`self.K2_DestroyActor`)
    (else
      (`KismetSystemLibrary.DelayUntilNextTick`)
      (goto _label))))

(event `self.Box.OnComponentBeginOverlap`
  (params (OverlappedComponent :type "PrimitiveComponent Object Reference") (OtherActor :type "Actor Object Reference") (OtherComp :type "PrimitiveComponent Object Reference") (OtherBodyIndex :type Integer) (bFromSweep :type Boolean) (SweepResult :type "HitResult Structure (by ref)"))
  (if (== (`GameplayStatics.GetObjectClass` OtherActor) (`self.Character`))
    (bind _asmain_character (cast `/Game/Common/MainCharacter` OtherActor))
    (`Character.LaunchCharacter` _asmain_character (0.0 0.0 1000.0) false false)
    (`self.K2_DestroyActor`)
    (else
      (`KismetSystemLibrary.PrintString` "FALSE"))))

(fn `UserConstructionScript`)